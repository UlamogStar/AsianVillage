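; BP_Bridge_01 is a bridge actor with swinging board pieces that flip when the third-person character enters one of three trigger volumes.
; All triggers play one timeline, whose BoardFlip track sets the relative pitch of four swing axis components together.
; The construction script configures InterpToMovement with the Duration variable and relative control points, the first two both using Location1.
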(event OnComponentBeginOverlap(Trigger(3))
  (params (OverlappedComponent :type Primitive%20Component%20Object%20Reference) (OtherActor :type Actor%20Object%20Reference) (OtherComp :type Primitive%20Component%20Object%20Reference) (OtherBodyIndex :type Integer) (bFromSweep :type Boolean) (SweepResult :type Hit%20Result%20Structure%20%28by%20ref%29))
  (Utilities|Casting|CastToBP_ThirdPersonCharacter OtherActor)
  (bind _boardflip (Timeline|Timeline Play)
    (:Update
      (Transformation|SetRelativeRotation (Variables|Default|GetBridgeswingGeo3Axis) (Math|Rotator|MakeRotator 0.0 _boardflip 0.0) false false))))

(event OnComponentBeginOverlap(Trigger(1))
  (params (OverlappedComponent :type Primitive%20Component%20Object%20Reference) (OtherActor :type Actor%20Object%20Reference) (OtherComp :type Primitive%20Component%20Object%20Reference) (OtherBodyIndex :type Integer) (bFromSweep :type Boolean) (SweepResult :type Hit%20Result%20Structure%20%28by%20ref%29))
  (Utilities|Casting|CastToBP_ThirdPersonCharacter OtherActor)
  (bind _boardflip (Timeline|Timeline Play)
    (:Update
      (Transformation|SetRelativeRotation (Variables|Default|GetBridgeswingGeo3Axis) (Math|Rotator|MakeRotator 0.0 _boardflip 0.0) false false))))

(event OnComponentBeginOverlap(Trigger(2))
  (params (OverlappedComponent :type Primitive%20Component%20Object%20Reference) (OtherActor :type Actor%20Object%20Reference) (OtherComp :type Primitive%20Component%20Object%20Reference) (OtherBodyIndex :type Integer) (bFromSweep :type Boolean) (SweepResult :type Hit%20Result%20Structure%20%28by%20ref%29))
  (Utilities|Casting|CastToBP_ThirdPersonCharacter OtherActor)
  (bind _boardflip (Timeline|Timeline Play)
    (:Update
      (Transformation|SetRelativeRotation (Variables|Default|GetBridgeswingGeo3Axis) (Math|Rotator|MakeRotator 0.0 _boardflip 0.0) false false))))

(fn ConstructionScript
  (bind _interptomovement (Variables|Default|GetInterpToMovement))
  (Variables|/Script/Engine.InterpToMovementComponent|SetControlPoints _interptomovement (Utilities|Array|MakeArray (Utilities|Struct|MakeInterpControlPoint (Variables|Default|GetLocation1) true) (Utilities|Struct|MakeInterpControlPoint (Variables|Default|GetLocation1) true) "" "" ""))
  (Variables|/Script/Engine.InterpToMovementComponent|SetDuration _interptomovement (Variables|Default|GetDuration)))