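; Turret actor that turns toward the third-person character on entering its TriggerZone and is set up to spawn short-lived projectiles from SpawnPoint.
; Overlap enables Tick and snaps rotation once, with no continuous tracking; exit disables Tick and resets RotationPoint.
; Firing is a self-looping RetriggerableDelay that every Tick restarts, holding off shots while ticking continues.
; BeginPlay's interpolated aim uses the turret's own location as target.
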(event OnComponentBeginOverlap(TriggerZone)
  (params (OverlappedComponent :type Primitive%20Component%20Object%20Reference) (OtherActor :type Actor%20Object%20Reference) (OtherComp :type Primitive%20Component%20Object%20Reference) (OtherBodyIndex :type Integer) (bFromSweep :type Boolean) (SweepResult :type Hit%20Result%20Structure%20%28by%20ref%29))
  (Utilities|FlowControl|Sequence
    (:then_0
      (Actor|Tick|SetActorTickEnabled true))
    (:then_1
      (bind _asbp_third_person_character (Utilities|Casting|CastToBP_ThirdPersonCharacter OtherActor))
      (Transformation|SetActorRotation (Math|Rotator|MakeRotator 0.0 (.pitch (Math|Rotator|FindLookatRotation (Transformation|GetActorLocation) (Transformation|GetActorLocation _asbp_third_person_character))) (.yaw (Math|Rotator|FindLookatRotation (Transformation|GetActorLocation) (Transformation|GetActorLocation _asbp_third_person_character))))))))

(event OnComponentEndOverlap(TriggerZone)
  (params (OverlappedComponent :type Primitive%20Component%20Object%20Reference) (OtherActor :type Actor%20Object%20Reference) (OtherComp :type Primitive%20Component%20Object%20Reference) (OtherBodyIndex :type Integer))
  (Actor|Tick|SetActorTickEnabled false)
  (Transformation|SetWorldRotation (Variables|Default|GetrotationPoint) "0, 0, 0" false false))

(event EventTick
  (params (DeltaSeconds :type Float%20%28single-precision%29))
  (bind _spawnpoint (Variables|Default|GetSpawnPoint))
  (Utilities|FlowControl|RetriggerableDelay 0.5 :!label _label)
  (bind _returnvalue (Game|SpawnActorfromClass "/Game/Blueprints/BP_Projectile_01.BP_Projectile_01_C" (Math|Transform|MakeTransform (Transformation|GetWorldLocation _spawnpoint) (Transformation|GetWorldRotation _spawnpoint) (Math|Conversions|ToVector(Float) (Variables|Default|GetProjectileScale))) "Undefined" "MultiplyWithRoot" 0 0))
  (Actor|SetLifeSpan _returnvalue 5.0)
  (goto _label))

(event EventBeginPlay
  (bind _returnvalue (Utilities|Time|GetWorldDeltaSeconds))
  (bind _returnvalue_2 (Transformation|GetActorRotation))
  (bind _returnvalue_3 (Transformation|GetActorLocation))
  (bind _returnvalue_4 (Transformation|GetActorLocation))
  (bind _returnvalue_5 (* 2e+01 5.0))
  (bind _returnvalue_6 (Math|Rotator|FindLookatRotation _returnvalue_3 _returnvalue_4))
  (bind _returnvalue_7 (Math|Interpolation|RInterpTo _returnvalue_2 _returnvalue_6 _returnvalue _returnvalue_5))
  (Transformation|SetWorldRotation (Variables|Default|GetrotationPoint) (Math|Rotator|MakeRotator 0.0 (Math|Float|Clamp(Float) (.pitch _returnvalue_7)) (.yaw _returnvalue_7)) false false)
  (Transformation|SetActorRotation (Math|Rotator|MakeRotator 0.0 0.0 (.yaw _returnvalue_7))))

(fn ConstructionScript)