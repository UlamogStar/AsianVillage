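; BP_Moving_Obj_Platform is a moving platform Blueprint driven by an InterpToMovement component.
; The Construction Script builds the component's control points from Location1 and Location2 as relative offsets and sets its travel time from Duration.
; The control point array has five slots, but the last three are unconnected, and the nodes built for Location3 to Location5 are unused.
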(fn ConstructionScript
  (bind _interptomovement (Variables|Default|GetInterpToMovement))
  (Variables|/Script/Engine.InterpToMovementComponent|SetControlPoints _interptomovement (Utilities|Array|MakeArray (Utilities|Struct|MakeInterpControlPoint (Variables|Default|GetLocation%201) true) (Utilities|Struct|MakeInterpControlPoint (Variables|Default|GetLocation%202) true) "" "" ""))
  (Variables|/Script/Engine.InterpToMovementComponent|SetDuration _interptomovement (Variables|Default|GetDuration)))